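; BPC_Health is a health component that tracks current and maximum health and a dead state.
; BeginPlay clears the dead flag and caches a BP_HUD actor reference, which the other graphs do not use.
; TakeDamage and GainHealth clamp health between zero and the maximum and are ignored once dead.
; Reaching zero calls Death, which uses a DoOnce to set the dead flag and fire the OnDeath dispatcher.
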(event EventBeginPlay
  (Variables|Default|SetCurrent%20Health (Variables|Default|GetCurrent%20Health))
  (Variables|Default|SetMax%20Health (Variables|Default|GetMax%20Health))
  (bind _returnvalue (Actor|GetActorOfClass "/Game/FrameWork/BP_HUD.BP_HUD_C"))
  (Variables|Default|SetHUD _returnvalue)
  (Variables|Default|SetDead false))

(event EventTick
  (params (DeltaSeconds :type Float%20%28single-precision%29)))

(fn TakeDamage
  (params (Damage :type Float%20%28double-precision%29))
  (if (not (Variables|Default|GetDead))
    (bind _output_get (Variables|Default|SetCurrent%20Health (Math|Float|Clamp(Float) (- (Variables|Default|GetCurrent%20Health) Damage) 0.0 (Variables|Default|GetMax%20Health))))
    (if (== _output_get 0.0)
      (CallFunction|Death))
    (return)))

(fn GainHealth
  (params (Health%20to%20Add :type Float%20%28double-precision%29))
  (if (not (Variables|Default|GetDead))
    (Variables|Default|SetCurrent%20Health (Math|Float|Clamp(Float) (+ Health%20to%20Add (Variables|Default|GetCurrent%20Health)) 0.0 (Variables|Default|GetMax%20Health)))
    (return)))

(fn Death
  (Utilities|FlowControl|DoOnce false
    (:Completed
      (Variables|Default|SetDead true)
      (Default|CallOnDeath))))