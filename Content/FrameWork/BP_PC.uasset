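; BP_PC is a player controller that relays the possessed character's life and the score to the HUD.
; On possess, it casts the pawn to BP_ThirdPersonCharacter and binds an event to its OnGetDamage dispatcher.
; DamageReceive and ScoreReceive cast the HUD to BP_HUD and pass it current and max life, or points.
; Nothing in this Blueprint calls or binds ScoreReceive by name.
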(event EventPossess
  (params (PossessedPawn :type Pawn%20Object%20Reference))
  (bind _asbp_third_person_character (Utilities|Casting|CastToBP_ThirdPersonCharacter PossessedPawn))
  (EventDispatchers|BindEventtoOnGetDamage _asbp_third_person_character (EventDispatchers|CreateEvent :!event DamageReceive)))

(fn ConstructionScript)

(fn DamageReceive
  (params (PawnCurretnLife :type Float%20%28double-precision%29) (PawnMaxLife :type Float%20%28double-precision%29))
  (bind _asbp_hud (Utilities|Casting|CastToBP_HUD (HUD|GetHUD)))
  (Default|ShowLife _asbp_hud PawnCurretnLife PawnMaxLife))

(fn ScoreReceive
  (params (Points :type Float%20%28double-precision%29))
  (bind _asbp_hud (Utilities|Casting|CastToBP_HUD (HUD|GetHUD)))
  (Default|ShowPoints _asbp_hud Points))