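; BP_Countdown is a game countdown that resumes from the saved value in BP_GameInstance, or starts at StartTime without a save.
; A looping one-second timer is set on BeginPlay, and CountdowTick decrements TimeRemaining and broadcasts updates.
; At zero it broadcasts completion and calls CheckIfLost on the player character.
; It also clears TimerHandle, but the node storing that handle is never executed.
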(event Custom|CountdowTick
  (bind _output_get (Variables|Default|SetTimeRemaining (- (Variables|Default|GetTimeRemaining) 1.0)))
  (Default|CallOnCountdownUpdated (Math|Float|Truncate _output_get))
  (if (<= _output_get 0.0)
    (Default|CallOnCountdownFinished)
    (Utilities|Time|ClearandInvalidateTimerbyHandle (Variables|Default|GetTimerHandle))
    (bind _asbp_third_person_character (Utilities|Casting|CastToBP_ThirdPersonCharacter (Game|Player|GetPlayerPawn 0)))
    (Default|CheckifLost _asbp_third_person_character)))

(event EventBeginPlay
  (bind _asbp_game_instance (Utilities|Casting|CastToBP_GameInstance (Game|GetGameInstance)))
  (Utilities|IsValid (Variables|/Game/Save_Load/BP_GameInstance.BP_GameInstance_C|GetCurrentLoadedSave _asbp_game_instance)
    (:Is%20Valid
      (Variables|Default|SetTimeRemaining (Variables|/Game/Save_Load/BP_Save.BP_Save_C|GetSavedCountdown (Variables|/Game/Save_Load/BP_GameInstance.BP_GameInstance_C|GetCurrentLoadedSave _asbp_game_instance))))
    (:Is%20Not%20Valid
      (Variables|Default|SetTimeRemaining (Variables|Default|GetStartTime))))
  (bind _returnvalue (Utilities|Time|SetTimerbyEvent (EventDispatchers|CreateEvent :!event Custom|CountdowTick) 1.0 true))
  (Default|CallOnCountdownUpdated))

(fn ConstructionScript)

(fn CountdownTick
  (params (Remaining :type Float%20%28double-precision%29)))