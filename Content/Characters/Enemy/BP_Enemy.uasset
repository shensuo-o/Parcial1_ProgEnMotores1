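; Enemy character that offers a looping waypoint route, senses actors through AI perception and can drop traps.
; On BeginPlay it offsets its waypoints by its own location, and NextWaypoint cycles through them.
; Perception updates set or clear the blackboard Target and write the sensed actor's location to Destination, with X and Y swapped.
; SpawnTrap spawns BP_TrapEnemy at TrapSpawnPoint and plays a sound.
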(event OnTargetPerceptionUpdated(AIPerception)
  (params (Actor :type Actor%20Object%20Reference) (Stimulus :type AI%20Stimulus%20Structure))
  (bind _returnvalue (Pawn|GetController))
  (bind _returnvalue_2 (AI|GetBlackboard _returnvalue))
  (Variables|Default|Setplayer Actor)
  (AI|Components|Blackboard|SetValueasObject _returnvalue_2 (Variables|Default|GetTarget) (Utilities|SelectObject Actor 0 (.bSuccessfullySensed (Utilities|Struct|BreakAIStimulus Stimulus))))
  (Class|KismetMathLibrary|VectorSet (Variables|Default|GetVector) (.Y (Math|Vector|BreakVector (Transformation|GetActorLocation (Variables|Default|Getplayer)))) (.X (Math|Vector|BreakVector (Transformation|GetActorLocation (Variables|Default|Getplayer)))) (.Z (Math|Vector|BreakVector (Transformation|GetActorLocation (Variables|Default|Getplayer)))))
  (AI|Components|Blackboard|SetValueasVector _returnvalue_2 (Variables|Default|GetDestination) (Variables|Default|GetVector)))

(event EventBeginPlay
  (for (_array_element _array_index) (Variables|Default|GetWaypoints)
    (Utilities|Array|SetArrayElem (Variables|Default|GetWaypoints) _array_index (+ _array_element (Transformation|GetActorLocation)))))

(fn ConstructionScript)

(fn NextWaypoint
  (bind _output_get (Variables|Default|SetDestinationIndex (Math|Integer|%(Integer) (+ (Variables|Default|GetDestinationIndex) 1) (Utilities|Array|Length (Variables|Default|GetWaypoints)))))
  (return (Utilities|Array|Get(acopy) (Variables|Default|GetWaypoints) _output_get)))

(fn SpawnTrap
  (Game|SpawnActorfromClass "/Game/Characters/Enemy/BP_TrapEnemy.BP_TrapEnemy_C" (Transformation|GetWorldTransform (Variables|Default|GetTrapSpawnPoint)) "Undefined" "MultiplyWithRoot" 0 0)
  (Audio|SpawnSoundatLocation "/Game/sonidos/tomato.tomato" (Transformation|GetActorLocation) "0, 0, 0" 1.0 1.0 0.0 0 0))