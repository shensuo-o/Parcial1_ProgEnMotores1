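; BP_LastCollectable is the final collectable pickup, hidden at start and revealed once the player character's Coleccionables count equals nine.
; It polls that count every Tick and toggles only visibility, leaving collision untouched.
; When a BP_ThirdPersonCharacter overlaps it, it plays a sound, increments the count and adds PointValue to the player's Points.
; It then sends the score to BP_PC through ScoreReceive and destroys itself.
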(event Collision|EventActorBeginOverlap
  (params (OtherActor :type Actor%20Object%20Reference))
  (bind _asbp_third_person_character (Utilities|Casting|CastToBP_ThirdPersonCharacter OtherActor))
  (Audio|SpawnSound2D "/Engine/VREditor/Sounds/UI/Click_on_Button_Cue.Click_on_Button_Cue" 1.0 1.0 0.0 0)
  (bind _output_get (Variables|/Game/ThirdPerson/Blueprints/BP_ThirdPersonCharacter.BP_ThirdPersonCharacter_C|SetColeccionables _asbp_third_person_character (+ (stale _output_get) 1)))
  (bind _asbp_third_person_character_2 (Utilities|Casting|CastToBP_ThirdPersonCharacter (Game|GetPlayerCharacter 0)))
  (bind _output_get_2 (Variables|/Game/ThirdPerson/Blueprints/BP_ThirdPersonCharacter.BP_ThirdPersonCharacter_C|SetPoints _asbp_third_person_character_2 (+ (Variables|/Game/ThirdPerson/Blueprints/BP_ThirdPersonCharacter.BP_ThirdPersonCharacter_C|GetPoints _asbp_third_person_character_2) (Variables|Default|GetPointValue))))
  (bind _asbp_pc (Utilities|Casting|CastToBP_PC (Game|GetInstigatorController _asbp_third_person_character_2)))
  (Default|ScoreReceive _asbp_pc _output_get_2)
  (Variables|Default|SetBPC_Collectable (Variables|Default|GetBPC_Collectable))
  (Actor|DestroyActor))

(event EventBeginPlay
  (Rendering|SetActorHiddenInGame true))

(event EventTick
  (params (DeltaSeconds :type Float%20%28single-precision%29))
  (bind _asbp_third_person_character (Utilities|Casting|CastToBP_ThirdPersonCharacter (Game|GetPlayerCharacter 0)))
  (if (== (Variables|/Game/ThirdPerson/Blueprints/BP_ThirdPersonCharacter.BP_ThirdPersonCharacter_C|GetColeccionables _asbp_third_person_character) 9)
    (Rendering|SetActorHiddenInGame false)))

(fn ConstructionScript)